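; Test enemy character that walks along the X axis in a random starting direction, with stun, knockback and death reactions.
; JumpStun toggles a squashed, paused state, while HitAction reverses direction and triggers Haywire.
; Non-platform collisions also knock it back into Haywire, which ends any stun and counts the hit for three seconds.
; Tick polls that counter, and two overlapping hits trigger a spinning death and destruction.
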(event Custom|WalkForward
  (Pawn|Input|AddMovementInput "1.000000,0.000000,0.000000" 1.0 false))

(event Custom|DeathEval
  (if (== (Variables|Default|GetHaywireHitCounter) 2)
    (Variables|Default|SetIsDying true)
    (Components|Movement|StopMovementImmediately (Variables|Character|GetCharacterMovement))
    (Collision|SetCollisionEnabled (Variables|Collision|GetCapsuleComponent) "NoCollision")
    (Character|LaunchCharacter "0.000000,0.000000,100.000000" false false)
    (Variables|/Script/Engine.CharacterMovementComponent|SetGravityScale (Variables|Character|GetCharacterMovement) 1e+01)
    (bind _newtrack_0 (Timeline|Timeline Play)
      (:Update
        (Transformation|SetActorRotation (Math|Rotator|Lerp(Rotator) (Variables|Default|GetCurrentRotation) "3780.000000,0.000000,0.000000" _newtrack_0))
        ;[0.15 0.1156 0.01889 0.5] fix
        (Utilities|FlowControl|Delay 3.0)
        (Actor|DestroyActor)))))

(event Custom|WalkBackward
  (Pawn|Input|AddMovementInput "-1.000000,0.000000,0.000000" 1.0 false))

(event Custom|Haywire
  (if (Variables|Default|GetPausing)
    (Variables|Default|SetPausing false)
    (CallFunction|JumpStun))
  (Math|Integer|IncrementInt (Variables|Default|GetHaywireHitCounter)
    (:%20%20
      (Niagara|SpawnSystemAttached "/Game/MAIN/NS_Vulnerable.NS_Vulnerable" (Variables|Default|GetNiagaraLocation) "None" "0, 0, 0" "0, 0, 0" "KeepRelativeOffset" true)
      ;[0.15 0.1204 0 0.5] fix "animation"
      (Utilities|FlowControl|Delay 3.0)
      (Math|Integer|DecrementInt (Variables|Default|GetHaywireHitCounter)))))

(event EventTick
  (params (DeltaSeconds :type Float%20%28single-precision%29))
  (CallFunction|DeathEval)
  (if (not (Variables|Default|GetPausing))
    (if (Variables|Default|GetRedirected)
      (CallFunction|WalkBackward)
      (else
        (CallFunction|WalkForward)))))

(event EventJumpStun
  (if (> (Variables|Default|GetSmooshCounter) 0)
    (CallFunction|Unsmoosh)
    (Variables|Default|SetPausing false)
    (else
      (CallFunction|Smoosh)
      (Variables|Default|SetPausing true))))

(event Collision|EventHit
  (params (MyComp :type Primitive%20Component%20Object%20Reference) (Other :type Actor%20Object%20Reference) (OtherComp :type Primitive%20Component%20Object%20Reference) (bSelfMoved :type Boolean) (HitLocation :type Vector :default "0, 0, 0") (HitNormal :type Vector :default "0, 0, 0") (NormalImpulse :type Vector :default "0, 0, 0") (Hit :type Hit%20Result%20Structure%20%28by%20ref%29))
  (bind _returnvalue (Actor|GetActorOfClass "/Game/MAIN/Environment/BP_Platform.BP_Platform_C"))
  (if (not (== _returnvalue Other))
    (Character|LaunchCharacter (Math|Vector|MakeVector (Math|Float|SelectFloat 2.5e+02 -2.5e+02 (< (.x (Pawn|Components|PawnMovement|GetLastInputVector (Variables|Character|GetCharacterMovement))) 0.0)) 0.0 2.5e+02) false false)
    ;[0 1 0.03945] Connect to see what happens!
    (Collision|SetCollisionEnabled (Variables|Collision|GetCapsuleComponent) "NoCollision")
    (CallFunction|Haywire)
    (Utilities|FlowControl|Delay 0.2)
    (Collision|SetCollisionEnabled (Variables|Collision|GetCapsuleComponent) "QueryAndPhysics")))

(event EventBeginPlay
  (Variables|Default|SetRedirected (Math|Random|RandomBool)))

(event EventHitAction
  (CallFunction|Haywire)
  (if (Variables|Default|GetRedirected)
    (Variables|Default|SetRedirected false)
    (else
      (Variables|Default|SetRedirected true))))

(event Input|GamepadEvents|DebugKeyGamepadDPadLeft
  (params (Key :type Key%20Structure :default "None") (ActionValue :type Input%20Action%20Value%20Structure)))

(event Input|KeyboardEvents|DebugKey1
  (params (Key :type Key%20Structure :default "None") (ActionValue :type Input%20Action%20Value%20Structure))
  (:Pressed
    (Development|PrintString "Hello")))

(event Input|KeyboardEvents|1
  (params (Key :type Key%20Structure :default "None")))

(fn ConstructionScript)

(fn Smoosh
  (Transformation|SetActorScale3D "1.000000,1.000000,1.000000")
  (Transformation|SetRelativeScale3D (Variables|Character|GetMesh) "0.700000,0.700000,0.450000")
  (Math|Integer|IncrementInt (Variables|Default|GetSmooshCounter)))

(fn Unsmoosh
  (Components|Capsule|SetCapsuleHalfHeight (Variables|Collision|GetCapsuleComponent) 7e+01 true)
  (Transformation|SetActorScale3D "1.000000,1.000000,1.000000")
  (Transformation|SetRelativeScale3D (Variables|Character|GetMesh) "0.700000,0.700000,0.700000")
  (Development|SetHiddeninGame (Variables|Collision|GetCapsuleComponent) false false)
  (Character|Jump)
  (Math|Integer|DecrementInt (Variables|Default|GetSmooshCounter)))