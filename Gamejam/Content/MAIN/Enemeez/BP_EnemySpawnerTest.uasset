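; Test enemy spawner actor that spawns a single BP_EnemyTest at its SpawnPoint location.
; BeginPlay caches an existing BP_EnemyTest found in the level as TargetActor.
; Tick calls RedirectBySpawnMessage on that cached enemy, spawns the new one, then increments SpawnCounter so the spawn runs only while the counter is not above zero.
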(event EventBeginPlay
  (bind _returnvalue (Actor|GetActorOfClass "/Game/MAIN/Enemeez/BP_EnemyTest.BP_EnemyTest_C"))
  (Variables|Default|SetTargetActor _returnvalue))

(event Collision|EventActorBeginOverlap
  (params (OtherActor :type Actor%20Object%20Reference)))

(event EventTick
  (params (DeltaSeconds :type Float%20%28single-precision%29))
  (if (not (> (Variables|Default|GetSpawnCounter) 0))
    (Class|BPIEnemyInteractTest|RedirectbySpawn(Message) (Variables|Default|GetTargetActor))
    (Game|SpawnActorfromClass "/Game/MAIN/Enemeez/BP_EnemyTest.BP_EnemyTest_C" (Math|Transform|MakeTransform (Transformation|GetWorldLocation (Variables|Default|GetSpawnPoint)) "0, 0, 0" "1.000000,1.000000,1.000000") "Undefined" "MultiplyWithRoot" 0 0)
    (Math|Integer|IncrementInt (Variables|Default|GetSpawnCounter))))

(fn ConstructionScript)