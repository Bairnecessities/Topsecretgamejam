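; BP_GalvoZD is the sprite-based Galvo character, with movement along its forward axis, jumping, ladder climbing and an attack.
; Climbing snaps it to the overlapping ladder in Flying mode and toggles that ladder's collision boxes by direction.
; Strong sideways input cancels climbing, restoring Falling mode and the starting Y depth.
; Canceling the combo input runs a sphere trace that messages the hit actor and briefly sets an attacking flag.
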(event Custom|Hit
  (bind _returnvalue (Transformation|GetActorLocation))
  (Variables|Default|SetIsAttacking true)
  (bind (_outhit _returnvalue_2) (Collision|SphereTraceForObjects _returnvalue _returnvalue 125.0 (Utilities|Array|MakeArray "ObjectTypeQuery7") false 0 "ForDuration"))
  (if _returnvalue_2
    (Class|BPIEnemyInteractTest|HitAction(Message) (.HitActor (Collision|BreakHitResult _outhit)) (.ImpactNormal (Collision|BreakHitResult _outhit)))
    (else
      (Development|PrintString "da fuck")))
  (Utilities|FlowControl|RetriggerableDelay 1.0)
  (Variables|Default|SetIsAttacking false))

(event Input|EnhancedActionEvents|EnhancedInputActionIA_Jump
  (params (ActionValue :type Boolean) (ElapsedSeconds :type Float%20%28double-precision%29) (TriggeredSeconds :type Float%20%28double-precision%29) (InputAction :type Input%20Action%20Object%20Reference :default "/Game/Input/Actions/IA_Jump.IA_Jump"))
  (:Triggered
    (Character|Jump))
  (:Canceled
    (Character|StopJumping :!label _label))
  (:Completed
    (goto _label)))

(event Input|EnhancedActionEvents|EnhancedInputActionIA_AimshotHipshotKOCombo
  (params (ActionValue :type Float%20%28double-precision%29) (ElapsedSeconds :type Float%20%28double-precision%29) (TriggeredSeconds :type Float%20%28double-precision%29) (InputAction :type Input%20Action%20Object%20Reference :default "/Game/MAIN/Inputz/IA_AimshotHipshotKOCombo.IA_AimshotHipshotKOCombo"))
  (:Canceled
    (CallFunction|Hit)))

(event Input|EnhancedActionEvents|EnhancedInputActionIA_Mover
  (params (ActionValue :type Vector%202D%20Structure) (ElapsedSeconds :type Float%20%28double-precision%29) (TriggeredSeconds :type Float%20%28double-precision%29) (InputAction :type Input%20Action%20Object%20Reference :default "/Game/Variant_SideScroller/Input/Actions/IA_Mover.IA_Mover"))
  (CallFunction|Move (.x ActionValue))
  (if (Variables|Default|GetCanClimb)
    (if (or (> (.y ActionValue) 0.3) (< (.y ActionValue) 0.3))
      (Variables|Default|SetIsClimbing true)
      (CallFunction|ClimbState (.y ActionValue))
      (if (or (> (.x ActionValue) 0.8) (< (.x ActionValue) -0.8))
        (CallFunction|CancelClimb)))))

(event EventBeginPlay
  (Variables|Default|SetStartingYLocation (.y (Transformation|GetActorLocation))))

(event EventTick
  (params (DeltaSeconds :type Float%20%28single-precision%29))
  (bind _returnvalue (Transformation|GetActorLocation))
  (Variables|Default|SetCurrentLocation (Math|Vector|MakeVector (.x _returnvalue) 0.0 (.z _returnvalue))))

(fn ConstructionScript)

(fn Move
  (params (ActionValueX :type Float%20%28double-precision%29))
  (Pawn|Input|AddMovementInput (Transformation|GetActorForwardVector) ActionValueX false))

(fn UpdateSpriteRotation
  (params (A :type Float%20%28double-precision%29))
  (Transformation|SetWorldRotation (Variables|Default|GetSprite) (Math|Rotator|SelectRotator "0.000000,-180.000000,0.000000" "0, 0, 0" (< A 0.0)) false false))

(fn ClimbState
  (params (ActionValueY :type Float%20%28single-precision%29))
  (bind _overlappingladder (Variables|Default|GetOverlappingLadder))
  (bind _overlappingladder_2 (Variables|Default|GetOverlappingLadder))
  (bind _overlappingladder_3 (Variables|Default|GetOverlappingLadder))
  (bind _overlappingladder_4 (Variables|Default|GetOverlappingLadder))
  (bind _fallboxtop (Variables|/Game/MAIN/Environment/BP_LadderTest.BP_LadderTest_C|GetFallBoxTop _overlappingladder_2))
  (bind _stopbox (Variables|/Game/MAIN/Environment/BP_LadderTest.BP_LadderTest_C|GetStopBox _overlappingladder))
  (bind _stopbox_2 (Variables|/Game/MAIN/Environment/BP_LadderTest.BP_LadderTest_C|GetStopBox _overlappingladder_3))
  (bind _fallboxtop_2 (Variables|/Game/MAIN/Environment/BP_LadderTest.BP_LadderTest_C|GetFallBoxTop _overlappingladder_4))
  (Utilities|FlowControl|Sequence
    (:then_0
      (Transformation|SetActorLocation (Math|Vector|MakeVector (.x (Transformation|GetActorLocation (Variables|Default|GetOverlappingLadder))) (+ (Variables|Default|GetStartingYLocation) 5e+01) (.z (Transformation|GetActorLocation))) false false)
      (Pawn|Components|CharacterMovement|SetMovementMode (Variables|Character|GetCharacterMovement) "MOVE_Flying" 0))
    (:then_1
      (Pawn|Input|AddMovementInput (Transformation|GetActorUpVector) ActionValueY false))
    (:then_2
      (if (> ActionValueY 0.0)
        (Collision|SetCollisionEnabled _fallboxtop_2 "QueryAndPhysics")
        (Development|SetHiddeninGame _fallboxtop_2 false false)
        (else
          (Collision|SetCollisionEnabled _fallboxtop "NoCollision")
          (Development|SetHiddeninGame _fallboxtop true false))))
    (:then_3
      (if (< ActionValueY 0.0)
        (Collision|SetCollisionEnabled _stopbox_2 "QueryAndPhysics")
        (Development|SetHiddeninGame _stopbox_2 false false)
        (else
          (Collision|SetCollisionEnabled _stopbox "NoCollision")
          (Development|SetHiddeninGame _stopbox true false))))))

(fn CancelClimb
  (bind _currentlocation (Variables|Default|GetCurrentLocation))
  (Variables|Default|SetIsClimbing false)
  (Pawn|Components|CharacterMovement|SetMovementMode (Variables|Character|GetCharacterMovement) "MOVE_Falling" 0)
  (Transformation|SetActorLocation (Math|Vector|MakeVector (.x _currentlocation) (Variables|Default|GetStartingYLocation) (.z _currentlocation)) false false))

(fn CanInteract
  (return false))