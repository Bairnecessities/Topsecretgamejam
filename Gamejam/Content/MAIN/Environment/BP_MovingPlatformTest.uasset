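; Test moving platform that shuttles its static mesh back and forth between its starting location and a target component.
; BeginPlay caches the actor location and plays a Timeline, whose Distance track lerps the mesh toward PlatformTargetLocation's world position without sweeping.
; When the Timeline finishes, its direction selects reverse or forward playback, looping the motion indefinitely.
; The target's world position is re-read on every update rather than cached.
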(event Custom|Forward
  (bind (_direction _distance) (Timeline|Timeline PlayFromStart)
    (:Update
      (Transformation|SetWorldLocation (Variables|Default|GetStaticMesh) (Math|Vector|Lerp(Vector) (Variables|Default|GetCurrentLocation) (Transformation|GetWorldLocation (Variables|Default|GetPlatformTargetLocation)) _distance) false false))
    (:Finished
      (switch Utilities|FlowControl|Switch|SwitchonETimelineDirection _direction
        (:Forward
          (CallFunction|Reverse))
        (:Backward
          (CallFunction|Forward))))))

(event Custom|Reverse
  (bind (_direction _distance) (Timeline|Timeline ReverseFromEnd)
    (:Update
      (Transformation|SetWorldLocation (Variables|Default|GetStaticMesh) (Math|Vector|Lerp(Vector) (Variables|Default|GetCurrentLocation) (Transformation|GetWorldLocation (Variables|Default|GetPlatformTargetLocation)) _distance) false false))
    (:Finished
      (switch Utilities|FlowControl|Switch|SwitchonETimelineDirection _direction
        (:Forward
          (CallFunction|Reverse))
        (:Backward
          (CallFunction|Forward))))))

(event EventBeginPlay
  (Variables|Default|SetCurrentLocation (Transformation|GetActorLocation))
  (CallFunction|Forward))

(fn ConstructionScript)