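; Melee attack actor component that deals damage to whatever stands just in front of its owner.
; The XCombo event sphere-traces a short distance along the owner's forward vector, ignoring the owner and drawing the trace for debugging.
; A hit actor with an AC_Health component receives fixed damage through TakeDamage.
; The XHold event is an empty stub.
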(event Custom|XCombo
  (bind _returnvalue (Components|GetOwner))
  (bind _returnvalue_2 (Transformation|GetActorLocation _returnvalue))
  (bind (_outhit _returnvalue_3) (Collision|SphereTraceForObjects _returnvalue_2 (+ _returnvalue_2 (* (Transformation|GetActorForwardVector _returnvalue) 2e+01)) 5e+01 (Utilities|Array|MakeArray "ObjectTypeQuery1" "ObjectTypeQuery3" "ObjectTypeQuery2" "ObjectTypeQuery6") false (Utilities|Array|MakeArray _returnvalue) "ForDuration"))
  (if _returnvalue_3
    (Utilities|IsValid (Actor|GetComponentbyClass (.HitActor (Collision|BreakHitResult _outhit)) "/Game/MAIN/ActorComponents/AC_Health.AC_Health_C")
      (:Is%20Valid
        (Default|TakeDamage (Actor|GetComponentbyClass (.HitActor (Collision|BreakHitResult _outhit)) "/Game/MAIN/ActorComponents/AC_Health.AC_Health_C") 2e+01)))))

(event Custom|XHold)