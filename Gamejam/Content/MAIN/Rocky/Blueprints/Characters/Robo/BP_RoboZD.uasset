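; Robot enemy character that patrols forward, turns at walls and reacts to stomps and hits.
; A stomp from BP_GalvoZD bounces that character and toggles the robot between squashed, paused and walking via JumpStun.
; HitAction knocks it back, flips it and triggers a timed Haywire state with vulnerability VFX and hopping.
; Tick drives walking and DeathEval, which starts a timeline spin and destroys the robot when two Haywire hits overlap.
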(event OnComponentBeginOverlap(WallDetector)
  (params (OverlappedComponent :type Primitive%20Component%20Object%20Reference) (OtherActor :type Actor%20Object%20Reference) (OtherComp :type Primitive%20Component%20Object%20Reference) (OtherBodyIndex :type Integer) (bFromSweep :type Boolean) (SweepResult :type Hit%20Result%20Structure%20%28by%20ref%29))
  ;[0.15 0 0.03526 0.5] Begin Overlap Component Wall Detector
  (Transformation|SetActorRotation (Math|Rotator|CombineRotators (Transformation|GetActorRotation) "0.000000,180.000000,0.000000")))

(event OnComponentHit(CapsuleComponent)
  (params (HitComponent :type Primitive%20Component%20Object%20Reference) (OtherActor :type Actor%20Object%20Reference) (OtherComp :type Primitive%20Component%20Object%20Reference) (NormalImpulse :type Vector :default "0, 0, 0") (Hit :type Hit%20Result%20Structure%20%28by%20ref%29))
  (if (Utilities|Operators|EqualEqual (.impactpoint Hit) (Transformation|GetWorldLocation (Variables|Default|GetHitImpactPoint)) 45.0)
    (if (not (Variables|Default|GetPausing))
      (Character|LaunchCharacter (Math|Vector|MakeVector (Math|Float|SelectFloat 2.5e+02 -2.5e+02 (< (.x (Pawn|Components|PawnMovement|GetLastInputVector (Variables|Character|GetCharacterMovement))) 0.0)) 0.0 2.5e+02) false false))))

(event OnComponentBeginOverlap(CapsuleComponent)
  (params (OverlappedComponent :type Primitive%20Component%20Object%20Reference) (OtherActor :type Actor%20Object%20Reference) (OtherComp :type Primitive%20Component%20Object%20Reference) (OtherBodyIndex :type Integer) (bFromSweep :type Boolean) (SweepResult :type Hit%20Result%20Structure%20%28by%20ref%29))
  (bind _asbp_galvo_zd (Utilities|Casting|CastToBP_GalvoZD OtherActor))
  (if (> (- (.z (Transformation|GetWorldLocation (Variables|/Game/MAIN/Rocky/Blueprints/Characters/Galvo/BP_GalvoZD.BP_GalvoZD_C|GetSmooshImpactPoint _asbp_galvo_zd))) (.z (Transformation|GetWorldLocation (Variables|Default|GetSmooshPoint)))) 0.0)
    (Character|LaunchCharacter _asbp_galvo_zd (Math|Vector|MakeVector (.x (Math|Vector|SelectVector "100.000000,0.000000,0.000000" "-100.000000,0.000000,0.000000" (> (.x (Transformation|GetVelocity (Game|Player|GetPlayerPawn 0))) 0.0))) 0.0 8e+02) false true)
    ;[0.15 0 0.03526 0.5] JumpStun
    (CallFunction|JumpStun)))

(event Custom|WalkForward
  (if (Variables|Default|GetIsHaywire)
    (Character|Jump))
  (Pawn|Input|AddMovementInput (Transformation|GetActorForwardVector) 1.0 false))

(event Custom|DeathEval
  (if (== (Variables|Default|GetHaywireHitCounter) 2)
    (Variables|Default|SetIsDying true)
    (Components|Movement|StopMovementImmediately (Variables|Character|GetCharacterMovement))
    (Collision|SetCollisionEnabled (Variables|Default|GetCapsuleComponent) "NoCollision")
    (Character|LaunchCharacter "0.000000,0.000000,100.000000" false false)
    (Variables|/Script/Engine.CharacterMovementComponent|SetGravityScale (Variables|Character|GetCharacterMovement) 1e+01)
    (bind _newtrack_0 (Timeline|Timeline Play)
      (:Update
        (Transformation|SetActorRotation (Math|Rotator|Lerp(Rotator) (Transformation|GetActorRotation) "3780.000000,0.000000,0.000000" _newtrack_0))
        ;[0.15 0.1156 0.01889 0.5] fix
        (Utilities|FlowControl|Delay 3.0)
        (Actor|DestroyActor)))))

(event Custom|Haywire
  ;[0.15 0 0.03526 0.5] Haywire
  (Math|Integer|IncrementInt (Variables|Default|GetHaywireHitCounter)
    (:%20%20
      (Variables|Default|SetIsHaywire true)
      (Niagara|SpawnSystemAttached "/Game/MAIN/NS_Vulnerable.NS_Vulnerable" (Variables|Default|GetNiagaraLocation) "None" "0, 0, 0" "0, 0, 0" "KeepRelativeOffset" true)
      ;[0.15 0.1204 0 0.5] fix "animation"
      (Utilities|FlowControl|Delay 3.0)
      (Math|Integer|DecrementInt (Variables|Default|GetHaywireHitCounter)
        (:%20%20
          (Variables|Default|SetIsHaywire false))))))

(event EventHitAction
  (params (HitNormal :type Vector :default "0, 0, 0"))
  ;[0.15 0 0.03526 0.5] Hit Action
  (Components|Movement|StopMovementImmediately (Variables|Character|GetCharacterMovement))
  (Character|LaunchCharacter (Math|Vector|MakeVector (Math|Float|SelectFloat 2e+02 -2e+02 (< (.x HitNormal) 0.0)) 0.0 4e+02) false false)
  (CallFunction|Haywire)
  (if (Variables|Default|GetPausing)
    (CallFunction|JumpStun))
  (Transformation|SetActorRotation (Math|Rotator|CombineRotators (Transformation|GetActorRotation) "0.000000,180.000000,0.000000")))

(event EventBeginPlay
  ;[0.15 0.1156 0.01889 0.5] Comment
)

(event EventTick
  (params (DeltaSeconds :type Float%20%28single-precision%29))
  (CallFunction|DeathEval)
  (if (not (Variables|Default|GetPausing))
    (CallFunction|WalkForward)))

(event EventJumpStun
  (if (> (Variables|Default|GetSmooshCounter) 0)
    (CallFunction|Unsmoosh)
    (Variables|Default|SetPausing false)
    ;[0.15 0.1156 0.01889 0.5] temp fix smoosh sprite sequencing
    (Collision|SetCollisionEnabled (Variables|Default|GetCapsuleComponent) "NoCollision")
    (Utilities|FlowControl|Delay 0.1)
    (Collision|SetCollisionEnabled (Variables|Default|GetCapsuleComponent) "QueryAndPhysics")
    (else
      (CallFunction|Smoosh)
      (Variables|Default|SetPausing true)
      (Collision|SetCollisionEnabled (Variables|Default|GetCapsuleComponent) "NoCollision")
      (Utilities|FlowControl|Delay 0.1)
      (Collision|SetCollisionEnabled (Variables|Default|GetCapsuleComponent) "QueryAndPhysics"))))

(fn ConstructionScript)

(fn Smoosh
  (Transformation|SetRelativeScale3D (Variables|Default|GetSprite) "1.250000,1.000000,0.750000")
  (Math|Integer|IncrementInt (Variables|Default|GetSmooshCounter)))

(fn Unsmoosh
  (Transformation|SetRelativeScale3D (Variables|Default|GetSprite) "1.000000,1.000000,1.000000")
  (Character|Jump)
  (Math|Integer|DecrementInt (Variables|Default|GetSmooshCounter)))